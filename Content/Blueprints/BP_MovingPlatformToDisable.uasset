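; BP_MovingPlatformToDisable is a platform actor that can be switched between present and absent in the level.
; Its Activate and Desactivate events run the same toggle, flipping root component visibility, propagated to children, and actor collision.
; Both events invert the current state instead of setting a fixed one, so the result depends on the starting state.
; The graph itself contains no movement logic.
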(event EventBeginPlay
  (|CallParentFunction) ; This node is disabled and will not be called.\nDrag off pins to build functionality.
)

(event EventTick
  (params (DeltaSeconds :type Float%20%28single-precision%29))
  (|CallParentFunction DeltaSeconds) ; This node is disabled and will not be called.\nDrag off pins to build functionality.
)

(event EventActivate
  (bind _rootcomponent (Variables|Transformation|GetRootComponent))
  (Rendering|SetVisibility _rootcomponent (not (Variables|/Script/Engine.SceneComponent|GetbVisible _rootcomponent)) true)
  (Collision|SetActorEnableCollision (not (Collision|GetActorEnableCollision))))

(event EventDesactivate
  (bind _rootcomponent (Variables|Transformation|GetRootComponent))
  (Rendering|SetVisibility _rootcomponent (not (Variables|/Script/Engine.SceneComponent|GetbVisible _rootcomponent)) true)
  (Collision|SetActorEnableCollision (not (Collision|GetActorEnableCollision))))

(fn ConstructionScript
  (|CallParentFunction))