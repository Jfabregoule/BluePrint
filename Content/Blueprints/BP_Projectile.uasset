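; Short-lived projectile that captures objects into the player's stock or places stocked ones back in the world.
; An overlap adds the other actor's class to BP_Player's StockedObjects and destroys that actor.
; A blocking hit spawns the last stocked class off-map, reads its bounds, then teleports it to the impact point, offset toward the camera.
; Both paths destroy the projectile and call StockedObjectsChange; otherwise it expires after a delay.
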(event OnComponentBeginOverlap(Collision)
  (params (OverlappedComponent :type Primitive%20Component%20Object%20Reference) (OtherActor :type Actor%20Object%20Reference) (OtherComp :type Primitive%20Component%20Object%20Reference) (OtherBodyIndex :type Integer) (bFromSweep :type Boolean) (SweepResult :type Hit%20Result%20Structure%20%28by%20ref%29))
  ;[0.07292 0.07292 0.07292] Get Object
  (bind _asbp_player (Utilities|Casting|CastToBP_Player (Game|GetPlayerCharacter 0)))
  (Utilities|Array|Add (Variables|/Game/Blueprints/BP_Player.BP_Player_C|GetStockedObjects _asbp_player) (Utilities|GetClass OtherActor))
  (Actor|DestroyActor OtherActor)
  (Actor|DestroyActor)
  (bind _asbp_player_2 (Utilities|Casting|CastToBP_Player (Game|GetPlayerCharacter 0)))
  (Default|StockedObjectsChange _asbp_player_2))

(event OnComponentHit(Collision)
  (params (HitComponent :type Primitive%20Component%20Object%20Reference) (OtherActor :type Actor%20Object%20Reference) (OtherComp :type Primitive%20Component%20Object%20Reference) (NormalImpulse :type Vector :default "0, 0, 0") (Hit :type Hit%20Result%20Structure%20%28by%20ref%29))
  ;[0.07292 0.07292 0.07292] Shoot Object
  (bind _asbp_player (Utilities|Casting|CastToBP_Player (Game|GetPlayerCharacter 0)))
  (if (Utilities|Array|IsNotEmpty (Variables|/Game/Blueprints/BP_Player.BP_Player_C|GetStockedObjects _asbp_player))
    (bind _returnvalue (Game|SpawnActorfromClass (Utilities|Array|Get(acopy) (Variables|/Game/Blueprints/BP_Player.BP_Player_C|GetStockedObjects _asbp_player) (- (Utilities|Array|Length (Variables|/Game/Blueprints/BP_Player.BP_Player_C|GetStockedObjects _asbp_player)) 1)) (Math|Transform|MakeTransform "-5000.000000,-5000.000000,-5000.000000") "AdjustIfPossibleButAlwaysSpawn" "MultiplyWithRoot" 0 0))
    (Transformation|SetActorLocation _returnvalue (+ (.ImpactPoint (Collision|BreakHitResult Hit)) (* (* (.BoxExtent (Collision|GetActorBounds _returnvalue true false)) (* (Math|Vector|GetForwardVector (Camera|GetCameraRotation (Game|GetPlayerCameraManager 0))) -1.0)) 1.5)) false true)
    (Utilities|Array|RemoveIndex (Variables|/Game/Blueprints/BP_Player.BP_Player_C|GetStockedObjects _asbp_player) (Utilities|Array|FindItem (Variables|/Game/Blueprints/BP_Player.BP_Player_C|GetStockedObjects _asbp_player) (Utilities|Array|Get(acopy) (Variables|/Game/Blueprints/BP_Player.BP_Player_C|GetStockedObjects _asbp_player) (- (Utilities|Array|Length (Variables|/Game/Blueprints/BP_Player.BP_Player_C|GetStockedObjects _asbp_player)) 1)))))
  (Actor|DestroyActor)
  (bind _asbp_player_2 (Utilities|Casting|CastToBP_Player (Game|GetPlayerCharacter 0)))
  (Default|StockedObjectsChange _asbp_player_2))

(event EventBeginPlay
  (Utilities|FlowControl|Delay 5.0)
  (Actor|DestroyActor))

(event Collision|EventActorBeginOverlap
  (params (OtherActor :type Actor%20Object%20Reference)))

(event EventTick
  (params (DeltaSeconds :type Float%20%28single-precision%29)))

(fn ConstructionScript)